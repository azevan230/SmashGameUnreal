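; Playable character Blueprint for Jammus in SmashUE, with Numpad 1, 2 and 3 switching it between Idle, Walk and Run.
; Each key changes the StateMachine state and sets whether and how fast the character moves.
; Tick applies movement input along X using OrientX, and polls the current state ID against LastStateId to swap to the matching Jammo montage only when the state changes.
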(event EventTick
  (params (DeltaSeconds :type Float%20%28single-precision%29))
  (if (Variables|Default|GetisMoving)
    (Pawn|Input|AddMovementInput (Math|Vector|MakeVector (+ (Variables|Default|GetOrientX) 0.0) 0.0 0.0) (Variables|Default|GetSpeed) false))
  (if (!= (Variables|Default|GetLastStateId) (Math|Conversions|ToInteger(Byte) (Variables|/Script/SmashUE.SmashCharacterStateMachine|GetCurrentStateID (Variables|Default|GetStateMachine))))
    (switch int (Math|Conversions|ToInteger(Byte) (Variables|/Script/SmashUE.SmashCharacterStateMachine|GetCurrentStateID (Variables|Default|GetStateMachine)))
      (:1
        (Animation|StopAnimMontage (Animation|GetCurrentMontage :!class /Script/Engine.Character))
        (Animation|PlayAnimMontage "/Game/Jammo/Animations/AM_Jammo_Idle.AM_Jammo_Idle" 1.0 "None")
        (Variables|Default|SetLastStateId "Idle"))
      (:2
        (Animation|StopAnimMontage (Animation|GetCurrentMontage :!class /Script/Engine.Character))
        (Animation|PlayAnimMontage "/Game/Jammo/Animations/AM_Jammo_Walk.AM_Jammo_Walk" 1.0 "None")
        (Variables|Default|SetLastStateId "Walk"))
      (:3
        (Animation|StopAnimMontage (Animation|GetCurrentMontage :!class /Script/Engine.Character))
        (Animation|PlayAnimMontage "/Game/Jammo/Animations/AM_Jammo_FastRun.AM_Jammo_FastRun" 1.0 "None")
        (Variables|Default|SetLastStateId "Run")))))

(event Input|KeyboardEvents|NumPadThree
  (params (Key :type Key%20Structure :default "None"))
  (:Pressed
    (Class|SmashCharacterStateMachine|ChangeState (Variables|Default|GetStateMachine) "Run")
    (Variables|Default|SetisMoving true)
    (Variables|Default|SetSpeed 1.0)))

(event Input|KeyboardEvents|NumPadOne
  (params (Key :type Key%20Structure :default "None"))
  (:Pressed
    (Class|SmashCharacterStateMachine|ChangeState (Variables|Default|GetStateMachine) "Idle")
    (Variables|Default|SetisMoving false)))

(event Input|KeyboardEvents|NumPadTwo
  (params (Key :type Key%20Structure :default "None"))
  (:Pressed
    (Class|SmashCharacterStateMachine|ChangeState (Variables|Default|GetStateMachine) "Walk")
    (Variables|Default|SetisMoving true)
    (Variables|Default|SetSpeed 0.6)))

(fn ConstructionScript)